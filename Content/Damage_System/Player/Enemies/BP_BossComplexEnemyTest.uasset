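; BP_BossComplexEnemyTest is a test boss enemy that heals itself on spawn and casts a lightning strike at the player when it sees a pawn.
; On sight, it waits two seconds, starts a looping timer bound to an empty custom event, then triggers the attacks component's delayed, damaging LightingStrike on the first player's character.
; The strike only fires while the damage system component reports the boss is not dead.
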(event `self.ReceiveBeginPlay`
  (`parent.ReceiveBeginPlay`)
  (`self.Heal` 150.0))

(event `CustomEvent`)

(event `self.PawnSensing.OnSeePawn`
  (params (Pawn :type "Pawn Object Reference"))
  (`|ExecutionSequence`
    (:`then_1`
      (`KismetSystemLibrary.Delay` 2.0)
      (`KismetSystemLibrary.K2_SetTimerDelegate` (delegate `CustomEvent`) 10.0 true)
      (if (not (`/Game/Damage_System/BPC_DamageSystem.IsDead` (`self.BPC_DamageSystem`)))
        (`/Game/Damage_System/Attacks/BPC_Attacks.LightingStrike` (`self.BPC_Attacks`) (`GameplayStatics.GetPlayerCharacter` 0) 1.0 20.0)))))

(fn `UserConstructionScript`
  (`parent.UserConstructionScript`))