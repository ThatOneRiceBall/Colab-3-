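; Base area-of-effect actor that finds pawns within a radius and reports each one through the OnAOEOverlapActor dispatcher.
; Trigger runs a one-shot sphere overlap at the actor's location, either when called or shortly after BeginPlay if TriggerOnBeginPlay is set.
; The query can exclude the instigator and optionally draws a debug sphere.
; It applies no damage itself, leaving the effect to whatever binds the dispatcher.
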(event `self.ReceiveBeginPlay`
  (if (`self.TriggerOnBeginPlay`)
    (`KismetSystemLibrary.Delay` 0.2)
    (`self.Trigger`)))

(event `Trigger`
  (`self.SpawnAOESphere`))

(event `SpawnAOESphere`
  (if (`self.DrawDebugSphere`)
    (`KismetSystemLibrary.DrawDebugSphere` (`self.K2_GetActorLocation`) (`self.Radius`) 12 (struct :`R` 1.0 :`G` 0.273434 :`B` 0.998566 :`A` 1.0) 2.0 1.0))
  (bind _outactors (`KismetSystemLibrary.SphereOverlapActors` (`self.K2_GetActorLocation`) (`self.Radius`) (`|MakeArray` "ObjectTypeQuery3" :!type "EObjectTypeQuery Enum") null (select `bool` (`self.IgnoreInstigator`) :`true` (`|MakeArray` (`self.GetInstigator`) :!type "Actor Object Reference"))))
  (for _array_element _outactors
    (`self.OnAOEOverlapActor` _array_element)))

(fn `UserConstructionScript`)