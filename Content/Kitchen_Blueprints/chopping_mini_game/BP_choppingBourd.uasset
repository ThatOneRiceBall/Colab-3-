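; Chopping board actor for the kitchen chopping mini-game that serves as an interaction point and ingredient spawner.
; An InteractCollision overlap by the player toggles the WB_Interact prompt and the chopping board interaction flag on BP_Player.
; Custom events spawn a carrot or mushroom just above the board, gated by DoOnce and a per-ingredient count.
; Each count only increments here, and DoOnce resets only after a successful spawn.
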(event `self.ReceiveBeginPlay`
  ; adds prompt to screen
  (bind _returnvalue (`|CreateWidget` "/Game/widgits/interact_widgit/WB_Interact.WB_Interact_C"))
  (set `self.NewVar` _returnvalue))

(event `self.interact collision.OnComponentBeginOverlap`
  (params (OverlappedComponent :type "PrimitiveComponent Object Reference") (OtherActor :type "Actor Object Reference") (OtherComp :type "PrimitiveComponent Object Reference") (OtherBodyIndex :type Integer) (bFromSweep :type Boolean) (SweepResult :type "HitResult Structure (by ref)"))
  (bind _returnvalue (`GameplayStatics.GetPlayerCharacter` 0))
  ; checks if overlapin with player character
  (if (== OtherActor _returnvalue)
    (`UserWidget.AddToViewport` (`self.NewVar`) 0)
    ; cast to player//check
    (bind _asbp_player (cast `/Game/Damage_System/Player/BP_Player` _returnvalue))
    (set `/Game/Damage_System/Player/BP_Player.is interacting with chopping bourd?` true _asbp_player)))

(event `self.interact collision.OnComponentEndOverlap`
  (params (OverlappedComponent :type "PrimitiveComponent Object Reference") (OtherActor :type "Actor Object Reference") (OtherComp :type "PrimitiveComponent Object Reference") (OtherBodyIndex :type Integer))
  (bind _returnvalue (`GameplayStatics.GetPlayerCharacter` 0))
  ; checks if overlapin with player character
  (if (== _returnvalue OtherActor)
    (`Widget.RemoveFromParent` (`self.NewVar`))
    ; cast to player//check
    (bind _asbp_player (cast `/Game/Damage_System/Player/BP_Player` _returnvalue))
    (set `/Game/Damage_System/Player/BP_Player.is interacting with chopping bourd?` false _asbp_player)))

(event `spawn_carot`
  (`self.spawn carrot`))

(event `spawn mushroom`
  (`self.spawn mooshroom`))

(fn `spawn carrot`
  (bind _returnvalue_location (`KismetMathLibrary.BreakTransform` (`self.GetTransform`)))
  (`/Engine/EditorBlueprintResources/StandardMacros.DoOnce` false :!label _label
    (:`Completed`
      (if (<= (`self.amount of carrots`) 0.0)
        (`|SpawnActorFromClass` "/Game/Kitchen_Blueprints/chopping_mini_game/vegtitables/Blueptints/BP_carrot.BP_carrot_C" (`KismetMathLibrary.MakeTransform` (+ _returnvalue_location (0.0 0.0 5.0)) (struct :`Yaw` 270.0)) "Undefined" "MultiplyWithRoot" null null)
        (set `self.amount of carrots` (+ (`self.amount of carrots`) 1.0))
        (goto _label :!via `Reset`)))))

(fn `spawn mooshroom`
  (bind _returnvalue_location (`KismetMathLibrary.BreakTransform` (`self.GetTransform`)))
  (`/Engine/EditorBlueprintResources/StandardMacros.DoOnce` false :!label _label
    (:`Completed`
      (if (<= (`self.amount of mushrooms`) 0.0)
        (`|SpawnActorFromClass` "/Game/Kitchen_Blueprints/chopping_mini_game/vegtitables/Blueptints/BP_Mushroom1.BP_Mushroom1_C" (`KismetMathLibrary.MakeTransform` (+ _returnvalue_location (0.0 0.0 5.0)) (struct :`Yaw` 270.0)) "Undefined" "MultiplyWithRoot" null null)
        (set `self.amount of mushrooms` (+ (`self.amount of mushrooms`) 1.0))
        (goto _label :!via `Reset`)))))

(fn `UserConstructionScript`)