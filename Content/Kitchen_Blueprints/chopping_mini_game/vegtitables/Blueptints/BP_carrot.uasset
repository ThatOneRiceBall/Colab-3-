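; BP_carrot is a choppable carrot for the kitchen chopping mini game.
; Each chop event flashes a short particle burst, then increments a cut counter through a DoOnce that resets until the fifth cut.
; That cut adds a Geometry Collection component, then after a delay decrements the carrot count on BP_choppingBourd and destroys the carrot.
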(event `chop`
  (bind _returnvalue (`GameplayStatics.SpawnEmitterAttached` "/Engine/Tutorial/SubEditors/TutorialAssets/TutorialParticleSystem.TutorialParticleSystem" (`self.GC_SM_Carrot1`) "None" (0.0 0.0 0.0) (struct) (0.1 0.1 0.1)))
  (`KismetSystemLibrary.Delay` 0.2)
  (`FXSystemComponent.SetEmitterEnable` _returnvalue "tutorialparticalsystem" false)
  (`/Engine/EditorBlueprintResources/StandardMacros.DoOnce` false :!label _label
    (:`Completed`
      (set `self.amount of cuts` (+ (`self.amount of cuts`) 1.0))
      (if (== (`self.amount of cuts`) 5.0)
        (`AddComponent|NODE_AddGeometryCollectionComponent-0`)
        (`KismetSystemLibrary.Delay` 2.0)
        (bind _returnvalue_2 (`GameplayStatics.GetActorOfClass` "/Game/Kitchen_Blueprints/chopping_mini_game/BP_choppingBourd.BP_choppingBourd_C"))
        (bind _asbp_chopping_bourd (cast `/Game/Kitchen_Blueprints/chopping_mini_game/BP_choppingBourd` _returnvalue_2))
        (set `/Game/Kitchen_Blueprints/chopping_mini_game/BP_choppingBourd.amount of carrots` (- (`/Game/Kitchen_Blueprints/chopping_mini_game/BP_choppingBourd.amount of carrots` _asbp_chopping_bourd) 1.0) _asbp_chopping_bourd)
        (`self.K2_DestroyActor`)
        (else
          (goto _label :!via `Reset`))))))

(fn `finnished chopping`)

(fn `UserConstructionScript`)