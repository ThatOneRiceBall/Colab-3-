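; Choppable mushroom for the kitchen chopping mini-game that breaks apart after five cuts.
; Each chop event plays a knife sound and advances a DoOnce-gated cut counter.
; The final cut flags it chopped, decrements BP_choppingBourd's mushroom count and swaps the static mesh for a geometry collection.
; A separate function, uncalled here, spawns TestCarrotChopped beside the board; LookAt returns empty text.
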(event `self.ReceiveBeginPlay`
  (`SceneComponent.SetHiddenInGame` (`self.GC_SM_Mushroom1`) true false))

(event `chop mushroom`
  (`GameplayStatics.PlaySound2D` "/Game/Sounds/Kitchen/knife-throw-1-105221.knife-throw-1-105221" 1.0 1.0 0.0 null null)
  ; checks amount of cuts (if==5 finnish chops)
  (`/Engine/EditorBlueprintResources/StandardMacros.DoOnce` false :!label _label
    (:`Completed`
      (set `self.amount of cuts` (+ (`self.amount of cuts`) 1.0))
      (if (== (`self.amount of cuts`) 5.0)
        (set `self.has been chopped` true)
        ; removes a carrot after cutting
        (bind _returnvalue (`GameplayStatics.GetActorOfClass` "/Game/Kitchen_Blueprints/chopping_mini_game/BP_choppingBourd.BP_choppingBourd_C"))
        (bind _asbp_chopping_bourd (cast `/Game/Kitchen_Blueprints/chopping_mini_game/BP_choppingBourd` _returnvalue))
        (set `/Game/Kitchen_Blueprints/chopping_mini_game/BP_choppingBourd.amount of mushrooms` (- (`/Game/Kitchen_Blueprints/chopping_mini_game/BP_choppingBourd.amount of mushrooms` _asbp_chopping_bourd) 1.0) _asbp_chopping_bourd)
        ; removes the SM and addes the broken geomatry
        (`ActorComponent.K2_DestroyComponent` (`self.StaticMesh`))
        (`AddComponent|NODE_AddGeometryCollectionComponent-0`)
        (`KismetSystemLibrary.Delay` 1.0)
        (else
          (goto _label :!via `Reset`))))))

(fn `LookAt`
  (returns (Message :type Text))
  (return ""))

(fn `spawn chopped mushroom`
  (bind _returnvalue (`GameplayStatics.GetActorOfClass` "/Game/Kitchen_Blueprints/chopping_mini_game/BP_choppingBourd.BP_choppingBourd_C"))
  (`/Engine/EditorBlueprintResources/StandardMacros.DoOnce` false :!label _label
    (:`Completed`
      (if true
        (bind _returnvalue_location (`KismetMathLibrary.BreakTransform` (`self.GetTransform` _returnvalue)))
        (`|SpawnActorFromClass` "/Game/Inventory/Items/TestCarrotChopped.TestCarrotChopped_C" (`KismetMathLibrary.MakeTransform` (+ _returnvalue_location (-50.0 0.0 5.0)) (struct :`Yaw` 180.0)) "Undefined" "MultiplyWithRoot" null null)
        (goto _label :!via `Reset`)))))

(fn `UserConstructionScript`)