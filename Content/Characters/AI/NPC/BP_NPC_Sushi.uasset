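; Sushi customer NPC that walks to the bar, shows its order and leaves when served or out of patience.
; Two chained timelines act as patience timers, turning the order text angry, then sending it away screaming.
; An overlap shows the interact widget and flags BP_Player's InteractedWithCustomer.
; On interaction after serving, matching meat and mushroom effect flags lead to an IsCooked check that picks a happy or screaming exit.
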(event `CustomerEnter2`
  (bind _ordertext (`self.OrderText`))
  ;[0.05119 0.15 0.09647 0.5] Makes the AI move into the Bar - Waits 5 Secs then switches to Angry Mode. - Waits 5 More Secs then Leaves. (Testing Times)
  (bind _returnvalue (`|CreateWidget` "/Game/widgits/interact_widgit/WB_Interact.WB_Interact_C"))
  (set `self.InteractText` _returnvalue)
  (if true
    (`|AIMoveTo` self (1665.354507 14.20835 85.0) null
      (:`OnSuccess`
        (`SceneComponent.SetVisibility` _ordertext true false)
        (`Timeline|Timeline` :!via `PlayFromStart` :!label _label
          (:`Finished`
            (`GameplayStatics.PlaySoundAtLocation` "/Game/Sounds/Kitchen/angry-roblox.angry-roblox" (`SceneComponent.K2_GetComponentLocation` (`self.CapsuleComponent`)) (struct) 1.0 1.0 0.0 null null null null)
            (`TextRenderComponent.K2_SetText` _ordertext (`self.Angry `))
            (`Timeline|Timeline_0` :!via `PlayFromStart` :!label _label_2
              (:`Finished`
                (`GameplayStatics.PlaySoundAtLocation` "/Game/Sounds/Kitchen/man-screaming-417689.man-screaming-417689" (`SceneComponent.K2_GetComponentLocation` (`self.CapsuleComponent`)) (struct) 1.0 1.0 0.0 null null null null)
                (`|AIMoveTo` self (2342.0 -450.0 85.0) null
                  (:`then`
                    (`SceneComponent.SetVisibility` (`self.OrderText`) false false)))))))))))

(event `self.Interact collision.OnComponentBeginOverlap`
  (params (OverlappedComponent :type "PrimitiveComponent Object Reference") (OtherActor :type "Actor Object Reference") (OtherComp :type "PrimitiveComponent Object Reference") (OtherBodyIndex :type Integer) (bFromSweep :type Boolean) (SweepResult :type "HitResult Structure (by ref)"))
  (bind _returnvalue (`GameplayStatics.GetPlayerCharacter` 0))
  ;[0.1451 0.2134 0.2552 0.7565] Displays "E to Interact" When inside the NPC's Collision
  (if (== OtherActor _returnvalue)
    (`UserWidget.AddToViewport` (`self.InteractText`) 0)
    (bind _asbp_player (cast `/Game/Damage_System/Player/BP_Player` _returnvalue))
    (set `/Game/Damage_System/Player/BP_Player.InteractedWithCustomer` true _asbp_player)))

(event `self.Interact collision.OnComponentEndOverlap`
  (params (OverlappedComponent :type "PrimitiveComponent Object Reference") (OtherActor :type "Actor Object Reference") (OtherComp :type "PrimitiveComponent Object Reference") (OtherBodyIndex :type Integer))
  (bind _returnvalue (`GameplayStatics.GetPlayerCharacter` 0))
  ;[0.1451 0.2134 0.2552 0.7565] Displays "E to Interact" When inside the NPC's Collision
  (if (== _returnvalue OtherActor)
    (`Widget.RemoveFromParent` (`self.InteractText`))
    (bind _asbp_player (cast `/Game/Damage_System/Player/BP_Player` _returnvalue))
    (set `/Game/Damage_System/Player/BP_Player.InteractedWithCustomer` false _asbp_player)))

(event `InteractWithNPC`
  ;[0.1448 0.15 0.05773 0.5] Checks if the Player has Interacted with the NPC - Makes NPC leave.
  (bind _asbp_player (cast `/Game/Damage_System/Player/BP_Player` (`GameplayStatics.GetPlayerCharacter` 0)))
  (if (`/Game/Damage_System/Player/BP_Player.ServedTest` _asbp_player)
    (set `self.ServedCorrect` true)
    (`|ExecutionSequence`
      (:`then_0`
        (bind _returnvalue (`GameplayStatics.GetActorOfClass` "/Game/Inventory/Items/Effects/Effect_HasMeetBeenUsed.Effect_HasMeetBeenUsed_C"))
        (bind _aseffect_has_meet_been_used (cast `/Game/Inventory/Items/Effects/Effect_HasMeetBeenUsed` _returnvalue)))
      (:`then_1`
        (bind _returnvalue_2 (`GameplayStatics.GetActorOfClass` "/Game/Inventory/Items/Effects/effect_HasMushroomBeenUsed.effect_HasMushroomBeenUsed_C"))
        (bind _aseffect_has_mushroom_been_used (cast `/Game/Inventory/Items/Effects/effect_HasMushroomBeenUsed` _returnvalue_2))))
    (if (== (`/Game/Inventory/Items/Effects/Effect_HasMeetBeenUsed.has meet been used` _aseffect_has_meet_been_used) (`/Game/Inventory/Items/Effects/effect_HasMushroomBeenUsed.has mushroom been used` _aseffect_has_mushroom_been_used))
      (if (`self.is cooked?`)
        (`|ExecutionSequence`
          (:`then_0`
            (`|ExecutionSequence`
              (:`then_0`
                (goto _label :!via `Stop`))
              (:`then_1`
                (goto _label_2 :!via `Stop`))
              (:`then_2`
                (`SceneComponent.SetVisibility` (`self.OrderText`) false false)
                (`|AIMoveTo` self (2342.0 -450.0 85.0) null
                  (:`then`
                    (`KismetSystemLibrary.PrintString` "one"))))))
          (:`then_1`
            (`/Engine/EditorBlueprintResources/StandardMacros.DoOnce` false
              (:`Completed`
                (`GameplayStatics.PlaySoundAtLocation` "/Game/Sounds/Kitchen/Ding.Ding" (`SceneComponent.K2_GetComponentLocation` (`self.CapsuleComponent`)) (struct) 1.0 1.0 0.0 null null null null)))))
        (else
          (`GameplayStatics.PlaySoundAtLocation` "/Game/Sounds/Kitchen/man-screaming-417689.man-screaming-417689" (`SceneComponent.K2_GetComponentLocation` (`self.CapsuleComponent`)) (struct) 1.0 1.0 0.0 null null null null)
          (`|AIMoveTo` self (2342.0 -450.0 85.0) null
            (:`then`
              (`SceneComponent.SetVisibility` (`self.OrderText`) false false)
              (`KismetSystemLibrary.PrintString` "two"))))))))

(fn `Serve`
  (locals (`IsCookedMeat?` :type Boolean)))

(fn `UserConstructionScript`)