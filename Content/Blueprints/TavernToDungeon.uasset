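; TavernToDungeon is a trigger Blueprint that lets the player travel from the tavern to the Dungeon_whiteboxing level.
; Box overlap creates a TavernToDungeon widget on screen, enables input for player 0 and sets InRange, without filtering the overlapping actor.
; Pressing Interact while InRange opens the level by object reference.
; Ending overlap disables input and removes the widget but leaves InRange set.
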(event `InputAction|Interact`
  (params (Key :type "Key Structure"))
  (:`Pressed`
    (if (`self.InRange`)
      (`GameplayStatics.OpenLevelBySoftObjectPtr` "/Game/Maps/Dungeon_whiteboxing.Dungeon_whiteboxing"))))

(event `self.Box.OnComponentBeginOverlap`
  (params (OverlappedComponent :type "PrimitiveComponent Object Reference") (OtherActor :type "Actor Object Reference") (OtherComp :type "PrimitiveComponent Object Reference") (OtherBodyIndex :type Integer) (bFromSweep :type Boolean) (SweepResult :type "HitResult Structure (by ref)"))
  (bind _returnvalue (`|CreateWidget` "/Game/Blueprints/TavernToDungeonWidget.TavernToDungeonWidget_C"))
  (bind _output_get (set `self.WidgetRef` _returnvalue))
  (`UserWidget.AddToViewport` _output_get 0)
  (`self.EnableInput` (`GameplayStatics.GetPlayerController` 0))
  (set `self.InRange` true))

(event `self.Box.OnComponentEndOverlap`
  (params (OverlappedComponent :type "PrimitiveComponent Object Reference") (OtherActor :type "Actor Object Reference") (OtherComp :type "PrimitiveComponent Object Reference") (OtherBodyIndex :type Integer))
  (`self.DisableInput` (`GameplayStatics.GetPlayerController` 0))
  (`Widget.RemoveFromParent` (`self.WidgetRef`)))

(fn `UserConstructionScript`)